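; BP_Button is a button pressed by motion controller overlap that fills a widget progress bar and ultimately starts a video.
; Each press lowers the mesh, swaps its material, plays a sound and adds progress.
; Tick slowly drains progress and raises the mesh until it can be pressed again.
; At full progress, it disables itself, hides the widget, and a timeline moves BP_Display and the button while opening the media source every update.
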(event `self.ReceiveTick`
  (params (DeltaSeconds :type "Float (single-precision)"))
  (bind _buttonmesh (`self.ButtonMesh`))
  (bind _currentprogress (`self.CurrentProgress`))
  ;[1 1 1] Decreasing progress bar percentage before it equal 100
  (if (and (>= _currentprogress 0.0) (<= _currentprogress 100.0))
    (`self.SetProgressBarPercentage` (- _currentprogress 0.05)))
  ;[1 1 1] Set button ready to press
  (if (`self.ButtonPressed`)
    (`SceneComponent.K2_AddRelativeLocation` _buttonmesh (0.0 0.0 0.2) false false)
    (if (>= (.z (`SceneComponent.RelativeLocation` _buttonmesh)) 50.0)
      (`PrimitiveComponent.SetMaterial` (`self.ButtonMesh`) 0 "/Game/VirtualReality/Materials/MI_SmallCubes.MI_SmallCubes")
      (set `self.ButtonPressed` false))))

(event `self.Box.OnComponentBeginOverlap`
  (params (OverlappedComponent :type "PrimitiveComponent Object Reference") (OtherActor :type "Actor Object Reference") (OtherComp :type "PrimitiveComponent Object Reference") (OtherBodyIndex :type Integer) (bFromSweep :type Boolean) (SweepResult :type "HitResult Structure (by ref)"))
  (bind _buttonmesh (`self.ButtonMesh`))
  ;[1 1 1] Pressing button and increasing progress bar percentage
  (cast `/Game/Blueprints/BP_MotionController` OtherActor)
  (if (`self.ButtonEnable`)
    (if (not (`self.ButtonPressed`))
      (`SceneComponent.K2_SetRelativeLocation` _buttonmesh (0.0 0.0 42.0) false false)
      (`PrimitiveComponent.SetMaterial` _buttonmesh 0 "/Game/Geometry/Meshes/CubeMaterial.CubeMaterial")
      (`self.SetProgressBarPercentage` (+ (`self.CurrentProgress`) 10.0))
      (`GameplayStatics.PlaySound2D` "/Game/SFX/S_Success.S_Success" 1.0 1.0 0.0 null null)
      (set `self.ButtonPressed` true)
      (`self.DisplayAppear`))))

(event `DisplayAppear`
  ;[1 1 1] Show display, hide button and start the video when progress bar percentage equal 100
  (if (>= (`self.CurrentProgress`) 100.0)
    (set `self.ButtonPressed` false)
    (`SceneComponent.SetVisibility` (`self.Widget`) false false)
    (set `self.ButtonEnable` false)
    (bind _outactors (`GameplayStatics.GetAllActorsOfClass` "/Game/Blueprints/BP_Display.BP_Display_C"))
    (bind (_direction _displayappearing _buttondisappearing) (`Timeline|MoveOblects`)
      (:`Update`
        (`self.K2_AddActorWorldTransform` (`|GetArrayItem` _outactors) (`KismetMathLibrary.MakeTransform` (`KismetMathLibrary.MakeVector` 0.0 0.0 _displayappearing)) false false)
        (`self.K2_AddActorWorldTransform` (`KismetMathLibrary.MakeTransform` (`KismetMathLibrary.MakeVector` 0.0 0.0 _buttondisappearing)))
        (`MediaPlayer.OpenSource` (`self.MediaPlayer_Ref`) "/Game/Movies/RV_FileMediaSource.RV_FileMediaSource")))))

(fn `SetProgressBarPercentage`
  (params (ExpressionToCalculate :type "Float (double-precision)"))
  (bind _output_get (set `self.CurrentProgress` ExpressionToCalculate))
  (bind _asw_progress_bar (cast `/Game/Blueprints/W_ProgressBar` (`WidgetComponent.GetUserWidgetObject` (`self.Widget`))))
  (set `/Game/Blueprints/W_ProgressBar.ProgressBarPercentage` (/ _output_get 100.0) _asw_progress_bar))

(fn `UserConstructionScript`)